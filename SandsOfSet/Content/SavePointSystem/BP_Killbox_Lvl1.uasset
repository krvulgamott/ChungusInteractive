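; BP_Killbox_Lvl1 is a killbox trigger that damages and respawns the 2D player character.
; Any overlap on its Box applies damage to player 0's BP_2DChar, without checking which actor entered.
; If Health is depleted it opens Lvl_FirstTemple; otherwise BP_ThirdPersonGameMode respawns the player.
; After respawning it shows a new W_HUD, then removes all widgets following a short delay.
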(event OnComponentBeginOverlap(Box)
  (params (OverlappedComponent :type Primitive%20Component%20Object%20Reference) (OtherActor :type Actor%20Object%20Reference) (OtherComp :type Primitive%20Component%20Object%20Reference) (OtherBodyIndex :type Integer) (bFromSweep :type Boolean) (SweepResult :type Hit%20Result%20Structure%20%28by%20ref%29))
  (bind _asbp_2dchar (Utilities|Casting|CastToBP_2DChar (Game|GetPlayerCharacter 0)))
  (Game|Damage|ApplyDamage _asbp_2dchar 1e+01 0 0)
  (if (<= (Variables|/Game/MainChar/BP_2DChar.BP_2DChar_C|GetHealth _asbp_2dchar) 0.0)
    (Game|OpenLevel(byName) "Lvl_FirstTemple")
    (else
      (bind _asbp_third_person_game_mode (Utilities|Casting|CastToBP_ThirdPersonGameMode (Game|GetGameMode)))
      (Default|RespawnPlayer _asbp_third_person_game_mode (Game|GetPlayerCharacter 0))
      (bind _returnvalue (UserInterface|CreateWidget "/Game/UI/W_HUD.W_HUD_C"))
      (bind _output_get (Variables|Default|SetHUD%20Widget _returnvalue))
      (UserInterface|Viewport|AddtoViewport _output_get 0)
      (Utilities|FlowControl|Delay 7.0)
      (Viewport|RemoveAllWidgets))))

(event EventBeginPlay)

(event Collision|EventActorBeginOverlap
  (params (OtherActor :type Actor%20Object%20Reference)))

(event EventTick
  (params (DeltaSeconds :type Float%20%28single-precision%29)))

(fn ConstructionScript)