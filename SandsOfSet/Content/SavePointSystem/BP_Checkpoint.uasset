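; Checkpoint actor that saves its own location as the player position when anything overlaps its Box.
; The overlap updates or creates a SaveGameObject and writes it to slot "1", though the existence check and load use an empty slot name.
; SaveCheckPoint separately saves a given position to slot "checkpoint" and prints a confirmation, but nothing here calls it.
; LoadCheckPoint is an empty stub.
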(event OnComponentBeginOverlap(Box)
  (params (OverlappedComponent :type Primitive%20Component%20Object%20Reference) (OtherActor :type Actor%20Object%20Reference) (OtherComp :type Primitive%20Component%20Object%20Reference) (OtherBodyIndex :type Integer) (bFromSweep :type Boolean) (SweepResult :type Hit%20Result%20Structure%20%28by%20ref%29))
  (bind _returnvalue (Transformation|GetActorLocation))
  (bind _returnvalue_2 (SaveGame|DoesSaveGameExist))
  (if _returnvalue_2
    (bind _returnvalue_3 (SaveGame|LoadGamefromSlot))
    (bind _assave_game_object (Utilities|Casting|CastToSaveGameObject _returnvalue_3))
    (Variables|/Game/SavePointSystem/SaveGameObject.SaveGameObject_C|SetPlayerPOS _assave_game_object _returnvalue)
    (SaveGame|SaveGametoSlot _assave_game_object "1")
    (else
      (bind _returnvalue_4 (SaveGame|CreateSaveGameObject "/Game/SavePointSystem/SaveGameObject.SaveGameObject_C"))
      (Variables|/Game/SavePointSystem/SaveGameObject.SaveGameObject_C|SetPlayerPOS _returnvalue_4 _returnvalue)
      (SaveGame|SaveGametoSlot _returnvalue_4 "1"))))

(event EventBeginPlay)

(event Collision|EventActorBeginOverlap
  (params (OtherActor :type Actor%20Object%20Reference)))

(event EventTick
  (params (DeltaSeconds :type Float%20%28single-precision%29)))

(fn ConstructionScript)

(fn SaveCheckPoint
  (params (PlayerPOS :type Vector))
  (bind _returnvalue (SaveGame|CreateSaveGameObject "/Game/SavePointSystem/SaveGameObject.SaveGameObject_C"))
  (Variables|/Game/SavePointSystem/SaveGameObject.SaveGameObject_C|SetPlayerPOS _returnvalue PlayerPOS)
  (bind _returnvalue_2 (SaveGame|SaveGametoSlot _returnvalue "checkpoint"))
  (if _returnvalue_2
    (Development|PrintText "CHECK POINT REACHED")))

(fn LoadCheckPoint)