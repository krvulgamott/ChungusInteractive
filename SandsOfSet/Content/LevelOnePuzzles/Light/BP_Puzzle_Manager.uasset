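; BP_Puzzle_Manager runs a level one light puzzle that opens a door when its braziers show the correct color code.
; Each Tick until solved, it compares every brazier piece's color index against the matching entry in the correct code array, stopping at the first mismatch.
; When all match, it latches a solved flag, casts the door reference to BP_LightDoorFIRE and calls its OnUse, with debug prints along the way.
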(event EventTick
  (params (DeltaSeconds :type Float%20%28single-precision%29))
  (if (not (Variables|Default|Getpuzzle_solved))
    (Variables|Default|Setis_correct true)
    (bind (_array_element _array_index) (Utilities|Array|ForEachLoopwithBreak (Variables|Default|Getbrazier_pieces) :!label _label)
      (:LoopBody
        (if (not (== (Variables|/Game/LevelOnePuzzles/Light/BP_fire_brazier_puzzle_piece.BP_fire_brazier_puzzle_piece_C|GetColorIndex _array_element) (Utilities|Array|Get(acopy) (Variables|Default|Getcorrect_code) _array_index)))
          (Variables|Default|Setis_correct false)
          (goto _label Break)))
      (:Completed
        (if (Variables|Default|Getis_correct)
          (Variables|Default|Setpuzzle_solved true)
          (Development|PrintString "Puzzle Solve")
          (bind _asbp_light_door_fire (Utilities|Casting|CastToBP_LightDoorFIRE (Variables|Default|Getdoor_to_open)))
          (Development|PrintString "OpenDoorPlz")
          (Default|OnUse _asbp_light_door_fire self))))))

(fn ConstructionScript)