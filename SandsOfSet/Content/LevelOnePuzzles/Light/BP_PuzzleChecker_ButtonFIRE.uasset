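; Fire puzzle checker button in the Level One light puzzle that opens a door when the color combination is correct.
; On Interact, it compares each puzzle piece's ColorIndex with the ColorCode entry at the same position.
; A match sends OnUseMessage to DoorToOpen once through Use_Interface, with debug prints reporting the result.
; A mismatch resets every piece to color index zero and refreshes its light.
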(event EventInteract
  (params (Interactor :type BP%202D%20Char%20Object%20Reference))
  (Variables|Default|SetisCorrect? true)
  ;[0.000983 0.1009 0.15 0.5] Places
  (bind (_array_element _array_index) (Utilities|Array|ForEachLoopwithBreak (Variables|Default|GetPuzzlePieces) :!label _label)
    (:LoopBody
      (if (!= (Variables|/Game/LevelOnePuzzles/Light/BP_fire_brazier_puzzle_piece.BP_fire_brazier_puzzle_piece_C|GetColorIndex _array_element) (Utilities|Array|Get(acopy) (Variables|Default|GetColorCode) _array_index))
        (Variables|Default|SetisCorrect? false)
        (goto _label Break)))
    (:Completed
      ;[0.15 0 0 0.5] Correct
      (if (Variables|Default|GetisCorrect?)
        ;[0.15 0.07837 0.002449 0.5] Open Door
        (Utilities|FlowControl|DoOnce false
          (:Completed
            (bind _doortoopen (Variables|Default|GetDoorToOpen)
              (:then
                (if (Utilities|DoesObjectImplementInterface _doortoopen "/Game/LevelOnePuzzles/Light/Use_Interface.Use_Interface_C")
                  (Class|UseInterface|OnUse(Message) _doortoopen self)
                  (Development|PrintString "Should Use")
                  (else
                    (Development|PrintString "Does Not Implement Use Interface"))))
              (:else
                (Development|PrintString "Door Does Not Exist")))))
        (else
          (bind _array_element_2 (Utilities|Array|ForEachLoopwithBreak (Variables|Default|GetPuzzlePieces))
            (:LoopBody
              (Variables|/Game/LevelOnePuzzles/Light/BP_fire_brazier_puzzle_piece.BP_fire_brazier_puzzle_piece_C|SetColorIndex _array_element_2 0)
              (Default|UpdateLightColor _array_element_2)
              (Development|PrintString "Should Fail"))))))))

(fn ConstructionScript)

(fn AddItem
  (params (Item :type Actor%20Object%20Reference))
  (return false))