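; BP_LightDoorFIREV2 is a door actor under the level-one light puzzles, built from a Cube and an OpenPos target.
; While IsMoving is true, Tick slides the Cube to OpenPos at constant speed with VInterpToConstant and prints a debug string.
; OnUse only sets IsMoving false when it is already false, so nothing in this Blueprint starts the motion.
; A delayed fixed-position move is left unconnected.
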(event EventOnUse
  (params (Actor :type Actor%20Object%20Reference))
  (if (not (Variables|Default|Getis_moving))
    (Variables|Default|Setis_moving false)
    (Development|PrintString "Door opening!")))

(event EventTick
  (params (DeltaSeconds :type Float%20%28single-precision%29))
  (if (Variables|Default|Getis_moving)
    (Transformation|SetWorldLocation (Variables|Default|GetCube) (Math|Interpolation|VInterptoConstant (Transformation|GetWorldLocation (Variables|Default|GetCube)) (Transformation|GetWorldLocation (Variables|Default|GetOpenPos)) DeltaSeconds 5e+02) false false)
    (Development|PrintString "Open")))

(event EventBeginPlay)

(fn ConstructionScript)