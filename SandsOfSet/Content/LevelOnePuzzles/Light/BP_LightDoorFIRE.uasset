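; BP_LightDoorFIRE is a door for the level one light puzzle that slides open when triggered.
; Its OnUse event opens a gate only when the passed actor is a BP_PuzzleChecker_ButtonFIRE.
; While the gate is open, Tick moves the Cube at constant speed toward the OpenPos location using VInterpToConstant.
; Nothing closes the gate again, and debug strings print on opening and failed casts.
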(event EventOnUse
  (params (Actor :type Actor%20Object%20Reference))
  (Utilities|Casting|CastToBP_PuzzleChecker_ButtonFIRE Actor
    (:then
      (Utilities|FlowControl|Gate true) ; enters at Open
    )
    (:CastFailed
      (Development|PrintString "Cast Failed"))))

(event EventTick
  (params (DeltaSeconds :type Float%20%28single-precision%29))
  (Utilities|FlowControl|Gate true
    (:Exit
      (Transformation|SetWorldLocation (Variables|Default|GetCube) (Math|Interpolation|VInterptoConstant (Transformation|GetWorldLocation (Variables|Default|GetCube)) (Transformation|GetWorldLocation (Variables|Default|GetOpenPos)) DeltaSeconds 6e+01) false false)
      (Development|PrintString "Open"))))

(fn ConstructionScript)