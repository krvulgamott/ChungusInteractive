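; A fire brazier puzzle piece for Level One that switches between four light and effect states when interacted with.
; Each Interact increments ColorIndex, wraps it back to zero after the last state, then calls UpdateLightColor.
; UpdateLightColor sets the point light's color and swaps the Niagara effect asset to match the index.
; AddItem always returns false, and the Blueprint itself holds no solution check.
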(event EventInteract
  (params (Interactor :type BP%202D%20Char%20Object%20Reference))
  ;[0.1332 0.05864 0.15 0.5] Switch
  (bind _result (Math|Integer|IncrementInt (Variables|Default|GetColorIndex))
    (:%20%20
      (if (<= _result 3)
        _
        (else
          (Variables|Default|SetColorIndex 0)))
      (CallFunction|UpdateLightColor))))

(fn ConstructionScript)

(fn UpdateLightColor
  (switch int (Variables|Default|GetColorIndex)
    (:0
      (Rendering|Components|Light|SetLightColor (Variables|Default|GetPointLight) "(R=1.000000,G=0.662961,B=0.416667,A=1.000000)" true)
      (Class|NiagaraComponent|SetAsset (Variables|Default|GetNiagara) "/Game/ParticleSystems/nia_SandyFootstep.nia_SandyFootstep" true))
    (:1
      (Rendering|Components|Light|SetLightColor (Variables|Default|GetPointLight) "(R=1.000000,G=0.835494,B=0.000000,A=1.000000)" true)
      (Class|NiagaraComponent|SetAsset (Variables|Default|GetNiagara) "/Game/Vefects/Free_Fire/Shared/Particles/NS_Fire_Floor_02_Simple.NS_Fire_Floor_02_Simple" true))
    (:2
      (Rendering|Components|Light|SetLightColor (Variables|Default|GetPointLight) "(R=1.000000,G=0.272765,B=0.000000,A=1.000000)" true)
      (Class|NiagaraComponent|SetAsset (Variables|Default|GetNiagara) "/Game/Vefects/Free_Fire/Shared/Particles/NS_Fire_Small.NS_Fire_Small" true))
    (:3
      (Rendering|Components|Light|SetLightColor (Variables|Default|GetPointLight) "(R=1.000000,G=0.072984,B=0.014233,A=1.000000)" true)
      (Class|NiagaraComponent|SetAsset (Variables|Default|GetNiagara) "/Game/Vefects/Free_Fire/Shared/Particles/NS_Fire_Medium.NS_Fire_Medium" true))))

(fn AddItem
  (params (Item :type Actor%20Object%20Reference))
  (return false))