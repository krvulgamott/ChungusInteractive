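; BP_Button is an interactable door button for the level one puzzles.
; On Interact it searches all BP_DoorCamera actors for those whose DoorValue matches its ButtonValue.
; Each match receives OpenDoor with the interactor and becomes player 0's view target through SetViewTargetWithBlend.
; AddItem always returns false, so the button accepts no items.
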(event EventInteract
  (params (Interactor :type BP%202D%20Char%20Object%20Reference))
  (bind _outactors (Actor|GetAllActorsOfClass "/Game/LevelOnePuzzles/DoorButton/BP_DoorCamera.BP_DoorCamera_C"))
  (bind _array_element (Utilities|Array|ForEachLoopwithBreak _outactors)
    (:LoopBody
      (if (== (Variables|/Game/LevelOnePuzzles/DoorButton/BP_DoorCamera.BP_DoorCamera_C|GetDoor%20Value _array_element) (Variables|Default|GetButtonValue))
        (Default|OpenDoor _array_element Interactor)
        (Game|Player|SetViewTargetwithBlend (Game|GetPlayerController 0) _array_element 0.0 "VTBlend_Linear" 0.0 false)))))

(fn ConstructionScript)

(fn AddItem
  (params (Item :type Actor%20Object%20Reference))
  (return false))