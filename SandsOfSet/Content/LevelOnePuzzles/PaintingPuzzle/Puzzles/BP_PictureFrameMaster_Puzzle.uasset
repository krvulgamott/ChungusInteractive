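; Rotatable picture frame for the painting puzzle, solved when every frame sits at its answer position.
; Interact sets Finalized by comparing the next position to PuzzleAnswer, then a timeline turns the picture 90 degrees and cycles FramePosition through four steps.
; Each frame runs a looping timer that checks all frames' Finalized flags and calls EVOPuzzleCompleted once all are true.
; Tick prints position and state for debugging.
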(event Custom|RotatePainting
  ;[0.15 0.1179 0.001821 0.5] Rotate Picture
  (if (not (Variables|Default|GetFrameMoving))
    (Variables|Default|SetFrameMoving true)
    (bind _rotation (Timeline|PaintingRotation PlayFromStart)
      (:Update
        (Transformation|SetRelativeRotation (Variables|Default|GetPicture) (Math|Rotator|MakeRotator 0.0 (Math|Float|Lerp (.pitch (Variables|Default|GetStartingRotationFrame)) (- (.pitch (Variables|Default|GetStartingRotationFrame)) 9e+01) _rotation) 0.0) false false))
      (:Finished
        (Variables|Default|SetStartingRotationFrame (Math|Rotator|MakeRotator 0.0 (Math|Float|Lerp (.pitch (Variables|Default|GetStartingRotationFrame)) (- (.pitch (Variables|Default|GetStartingRotationFrame)) 9e+01) _rotation) 0.0))
        (Variables|Default|SetFrameMoving false)
        (bind _result (Math|Integer|IncrementInt (Variables|Default|GetFramePosition))
          (:%20%20
            (bind _output_get (Variables|Default|SetFramePosition _result))
            (if (> _output_get 3)
              (Variables|Default|SetFramePosition 0))))))))

(event Custom|PuzzleCheck
  (Variables|Default|SetPuzzleSolved true)
  (for _array_element (Variables|Default|GetAllPictureFrames)
    (if (not (Variables|BP_PictureFrameMaster_Puzzle_C|GetFinalized _array_element))
      (Variables|Default|SetPuzzleSolved false)))
  (if (Variables|Default|GetPuzzleSolved)
    (Utilities|Time|ClearandInvalidateTimerbyHandle (stale EventBeginPlay _returnvalue))
    (Default|CallEVOPuzzleCompleted)))

(event EventInteract
  (params (Interactor :type BP%202D%20Char%20Object%20Reference))
  (if (== (+ (Variables|Default|GetFramePosition) 1) (Variables|Default|GetPuzzleAnswer))
    (Variables|Default|SetFinalized true)
    (CallFunction|RotatePainting)
    (else
      (Variables|Default|SetFinalized false)
      (CallFunction|RotatePainting))))

(event EventBeginPlay
  ;[0.15 0.001047 0.0121 0.5] Interact / Event Play
  (Variables|Default|SetStartingRotationFrame (Variables|/Script/Engine.SceneComponent|GetRelativeRotation (Variables|Default|GetPicture)))
  (bind _outactors (Actor|GetAllActorsOfClass "BP_PictureFrameMaster_Puzzle_C"))
  (Variables|Default|SetAllPictureFrames _outactors)
  (bind _returnvalue (Utilities|Time|SetTimerbyEvent (delegate Custom|PuzzleCheck) 0.25 true)))

(event EventTick
  (params (DeltaSeconds :type Float%20%28single-precision%29))
  (Development|PrintString (Utilities|String|ToString(Integer) (Variables|Default|GetFramePosition)) true true "(R=0.000000,G=0.660000,B=1.000000,A=1.000000)" DeltaSeconds)
  (Development|PrintString (Utilities|String|ToString(Boolean) (Variables|Default|GetFinalized)) true true "(R=0.000000,G=0.660000,B=1.000000,A=1.000000)" DeltaSeconds))

(fn ConstructionScript
  (|CallParentFunction))