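; BP_MoveableCube is a pushable block for the level one puzzles that only moves physically while the player is pushing it.
; Separate X-axis and Y-axis collision components detect overlaps with BP_2DChar.
; Overlap begin enables physics simulation on the Cube and sets the character's IsPushing flag, and overlap end turns both off.
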(event OnComponentBeginOverlap(YAxisCollision)
  (params (OverlappedComponent :type Primitive%20Component%20Object%20Reference) (OtherActor :type Actor%20Object%20Reference) (OtherComp :type Primitive%20Component%20Object%20Reference) (OtherBodyIndex :type Integer) (bFromSweep :type Boolean) (SweepResult :type Hit%20Result%20Structure%20%28by%20ref%29))
  ;[0 0.01472 0.15 0.5] Y Axis Collision
  (bind _asbp_2dchar (Utilities|Casting|CastToBP_2DChar OtherActor))
  (Physics|SetSimulatePhysics (Variables|Default|GetCube) true)
  (Variables|/Game/MainChar/BP_2DChar.BP_2DChar_C|SetIsPushing? _asbp_2dchar true))

(event OnComponentEndOverlap(YAxisCollision)
  (params (OverlappedComponent :type Primitive%20Component%20Object%20Reference) (OtherActor :type Actor%20Object%20Reference) (OtherComp :type Primitive%20Component%20Object%20Reference) (OtherBodyIndex :type Integer))
  ;[0 0.01472 0.15 0.5] Y Axis Collision
  (bind _asbp_2dchar (Utilities|Casting|CastToBP_2DChar OtherActor))
  (Physics|SetSimulatePhysics (Variables|Default|GetCube) false)
  (Variables|/Game/MainChar/BP_2DChar.BP_2DChar_C|SetIsPushing? _asbp_2dchar false))

(event OnComponentBeginOverlap(XAxisCollision)
  (params (OverlappedComponent :type Primitive%20Component%20Object%20Reference) (OtherActor :type Actor%20Object%20Reference) (OtherComp :type Primitive%20Component%20Object%20Reference) (OtherBodyIndex :type Integer) (bFromSweep :type Boolean) (SweepResult :type Hit%20Result%20Structure%20%28by%20ref%29))
  ;[1 0.2917 0.2917 0.5] X Axis Collision
  (bind _asbp_2dchar (Utilities|Casting|CastToBP_2DChar OtherActor))
  (Physics|SetSimulatePhysics (Variables|Default|GetCube) true)
  (Variables|/Game/MainChar/BP_2DChar.BP_2DChar_C|SetIsPushing? _asbp_2dchar true))

(event OnComponentEndOverlap(XAxisCollision)
  (params (OverlappedComponent :type Primitive%20Component%20Object%20Reference) (OtherActor :type Actor%20Object%20Reference) (OtherComp :type Primitive%20Component%20Object%20Reference) (OtherBodyIndex :type Integer))
  ;[1 0.2917 0.2917 0.5] X Axis Collision
  (bind _asbp_2dchar (Utilities|Casting|CastToBP_2DChar OtherActor))
  (Physics|SetSimulatePhysics (Variables|Default|GetCube) false)
  (Variables|/Game/MainChar/BP_2DChar.BP_2DChar_C|SetIsPushing? _asbp_2dchar false))

(fn ConstructionScript)