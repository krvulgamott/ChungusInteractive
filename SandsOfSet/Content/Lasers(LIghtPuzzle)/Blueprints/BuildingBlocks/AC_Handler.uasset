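; Laser puzzle component that decides when its owning actor activates or deactivates from the lasers hitting it.
; It tracks incoming lasers, drops filtered colors and tests the rest against color rules, individually or additively merged.
; Results propagate to sibling BPI_Lasers components and handler dispatchers, immediately or after a reversible timer that broadcasts its alpha.
; Forced changes can bypass the rules, with activation still requiring all linked external components to be active.
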(event Custom|CE_TimerFinishedDeactivate
  (bind _array_element (Utilities|ForEachComponent)
    (:LoopBody
      (Class|BPILasers|LaserStopHitting(Message) _array_element (stale EventLaserStopHitting Input)))
    (:Completed
      (CallFunction|ComponentColorChange (stale EventLaserStopHitting Input))
      (Default|CallDectivateHandler self))))

(event Custom|CE_ActivateOverride
  (if (not (Utilities|UseTimer))
    (bind _array_element (Utilities|ForEachComponent)
      (:LoopBody
        (Class|BPILasers|LaserStartHitting(Message) _array_element (stale EventLaserStartHitting Input) (stale EventLaserStartHitting Hit%20Info)))
      (:Completed
        (Default|CallActivateHandler self)))
    (else
      (Variables|Timer|SetReverseTimer false)
      (CallFunction|StartTimer false))))

(event Custom|CE_DeactivateOverride
  (if (not (Utilities|UseTimer))
    (bind _array_element (Utilities|ForEachComponent)
      (:LoopBody
        (Class|BPILasers|LaserStopHitting(Message) _array_element (stale EventLaserStopHitting Input)))
      (:Completed
        (CallFunction|ComponentColorChange (stale EventLaserStopHitting Input))
        (Default|CallDectivateHandler self)))
    (else
      (Variables|Timer|SetReverseTimer true)
      (CallFunction|StartTimer false))))

(event Custom|CE_TimerFinishedActivate
  (bind _array_element (Utilities|ForEachComponent)
    (:LoopBody
      (Class|BPILasers|LaserStartHitting(Message) _array_element (stale EventLaserStartHitting Input) (stale EventLaserStartHitting Hit%20Info)))
    (:Completed
      (Default|CallActivateHandler self))))

(event Custom|CE_Ext_TimerDeactivate
  (bind _array_element (Utilities|ForEachComponent)
    (:LoopBody
      (Class|BPILasers|ForceDeactivation(Message) _array_element (stale EventForceDeactivation ApplyConditions)))
    (:Completed
      (CallFunction|ComponentColorChange 0)
      (Default|CallDectivateHandler self))))

(event Custom|CE_Ext_TimerActivate
  (bind _array_element (Utilities|ForEachComponent)
    (:LoopBody
      (Class|BPILasers|ForceActivation(Message) _array_element (stale EventForceActivation ApplyConditions)))
    (:Completed
      (Default|CallActivateHandler self))))

(event EventBeginPlay
  (Utilities|FlowControl|Sequence
    (:then_0
      (bind _output_get (Variables|Strorage|SetLinked%20Components (Class|Actor|GetComponentsbyInterface (Components|GetOwner) "/Game/Lasers(LIghtPuzzle)/Blueprints/BuildingBlocks/BPI_Lasers.BPI_Lasers_C")))
      (Utilities|Array|RemoveItem _output_get self)
      (for _array_element (Actor|GetComponentsByClass (Components|GetOwner) "/Script/Engine.StaticMeshComponent")
        (Collision|SetCollisionResponsetoChannel _array_element "ECC_GameTraceChannel1" (select (Variables|Conditions|GetIsBlocking) "ECR_Block" "ECR_Overlap"))))
    (:then_1
      (if (Variables|Conditions|GetInvert%20System)
        (for _array_element_2 (Actor|GetComponentsByClass (Components|GetOwner) "/Game/Lasers(LIghtPuzzle)/Blueprints/BuildingBlocks/SC_Emitter.SC_Emitter_C")
          (Default|SetLaserColor _array_element_2)
          (Default|LaserStopHitting _array_element_2))))
    (:then_2
      (for (_array_element_3 _array_index) (Variables|Lasers|GetLaserRules)
        (Utilities|Array|SetArrayElem (Variables|Lasers|GetLaserRules) _array_index (Utilities|SetAlphato1 _array_element_3)))
      (for (_array_element_4 _array_index_2) (Variables|Lasers|GetLaserFilter)
        (Utilities|Array|SetArrayElem (Variables|Lasers|GetLaserFilter) _array_index_2 (Utilities|SetAlphato1 _array_element_4))))))

(event EventLaserUpdateHitting
  (params (Input :type A%20Laser%20Object%20Reference) (Hit%20Info :type Hit%20Result%20Structure))
  (bind _array_element (Utilities|ForEachComponent)
    (:LoopBody
      (Class|BPILasers|LaserUpdateHitting(Message) _array_element Input Hit%20Info))))

(event EventLaserStartHitting
  (params (Input :type A%20Laser%20Object%20Reference) (Hit%20Info :type Hit%20Result%20Structure))
  (CallFunction|LaserAdded Input)
  (Utilities|IsNotLocked
    (:Not%20Locked
      (if (CallFunction|CanActivate)
        (if (not (Utilities|UseTimer))
          (bind _array_element (Utilities|ForEachComponent)
            (:LoopBody
              (Class|BPILasers|LaserStartHitting(Message) _array_element Input Hit%20Info))
            (:Completed
              (Default|CallActivateHandler self)))
          (else
            (Variables|Timer|SetReverseTimer false)
            (CallFunction|StartTimer false)))))))

(event EventLaserStopHitting
  (params (Input :type A%20Laser%20Object%20Reference))
  (CallFunction|LaserRemoved Input)
  (Utilities|IsNotLocked
    (:Not%20Locked
      (if (not (CallFunction|CanActivate))
        (if (not (Utilities|UseTimer))
          (bind _array_element (Utilities|ForEachComponent)
            (:LoopBody
              (Class|BPILasers|LaserStopHitting(Message) _array_element Input))
            (:Completed
              (CallFunction|ComponentColorChange Input)
              (Default|CallDectivateHandler self)))
          (else
            (Variables|Timer|SetReverseTimer true)
            (CallFunction|StartTimer false)))
        (else
          (CallFunction|ComponentColorChange Input))))))

(event EventIntermediateChange
  (params (Modified :type A%20Laser%20Object%20Reference))
  (CallFunction|RecalculateColors Modified))

(event EventForceActivation
  (params (ApplyConditions :type Boolean))
  (if ApplyConditions
    (if (CallFunction|CanActivate)
      (if (CallFunction|AreAllCompsActivated) :!label _label
        (if (not (Utilities|UseTimer))
          (bind _array_element (Utilities|ForEachComponent)
            (:LoopBody
              (Class|BPILasers|ForceActivation(Message) _array_element ApplyConditions))
            (:Completed
              (Default|CallActivateHandler self)))
          (else
            (Variables|Timer|SetReverseTimer false)
            (CallFunction|StartTimer true)))))
    (else
      (goto _label))))

(event EventForceDeactivation
  (params (ApplyConditions :type Boolean))
  (if ApplyConditions
    (if (not (CallFunction|CanActivate))
      (if (not (Utilities|UseTimer)) :!label _label
        (bind _array_element (Utilities|ForEachComponent)
          (:LoopBody
            (Class|BPILasers|ForceDeactivation(Message) _array_element ApplyConditions))
          (:Completed
            (CallFunction|ComponentColorChange 0)
            (Default|CallDectivateHandler self)))
        (else
          (Variables|Timer|SetReverseTimer true)
          (CallFunction|StartTimer true))))
    (else
      (goto _label))))

(fn LaserAdded
  (params (NewItem :type A%20Laser%20Object%20Reference%20%28by%20ref%29))
  (Utilities|Array|AddUnique (Variables|Strorage|GetLasersInQueue) NewItem)
  (if (not (CallFunction|IsLaserFiltered NewItem))
    (Utilities|Array|AddUnique (Variables|Strorage|GetFilteredLasers) NewItem)
    (if (or (Utilities|Enum|Equal(Enum) (Variables|Colors|GetUsedColor) "NewEnumerator2") (Variables|Colors|GetCanMergeColor))
      (Variables|Colors|SetMerged%20Color (+ (Variables|Colors|GetMerged%20Color) (Variables|/Game/Lasers(LIghtPuzzle)/Blueprints/BuildingBlocks/A_Laser.A_Laser_C|GetColorOverride NewItem))))))

(fn LaserRemoved
  (params (NewItem :type A%20Laser%20Object%20Reference%20%28by%20ref%29))
  (Utilities|Array|RemoveItem (Variables|Strorage|GetLasersInQueue) NewItem)
  (if (not (CallFunction|IsLaserFiltered NewItem))
    (Utilities|Array|RemoveItem (Variables|Strorage|GetFilteredLasers) NewItem)
    (if (or (Utilities|Enum|Equal(Enum) (Variables|Colors|GetUsedColor) "NewEnumerator2") (Variables|Colors|GetCanMergeColor))
      (Variables|Colors|SetMerged%20Color (- (Variables|Colors|GetMerged%20Color) (Variables|/Game/Lasers(LIghtPuzzle)/Blueprints/BuildingBlocks/A_Laser.A_Laser_C|GetColorOverride NewItem))))))

(fn GetVisibleColor
  (bind _lasersinqueue (Variables|Strorage|GetLasersInQueue))
  (Utilities|FlowControl|Sequence
    (:then_0
      (switch Utilities|FlowControl|Switch|SwitchonE_ColorSelection (Variables|Colors|GetUsedColor)
        (:NewEnumerator0
          (Variables|Colors|SetPassByColor (Variables|/Game/Lasers(LIghtPuzzle)/Blueprints/BuildingBlocks/A_Laser.A_Laser_C|GetColorOverride (Utilities|Array|Get(acopy) (Variables|Strorage|GetLasersInQueue)))))
        (:NewEnumerator1
          (Variables|Colors|SetPassByColor (Variables|/Game/Lasers(LIghtPuzzle)/Blueprints/BuildingBlocks/A_Laser.A_Laser_C|GetColorOverride (Utilities|Array|Get(acopy) _lasersinqueue (Utilities|Array|LastIndex _lasersinqueue)))))
        (:NewEnumerator2
          (Variables|Colors|SetPassByColor (CallFunction|GetMergedColor)))))
    (:then_1
      (return (Variables|Colors|GetPassByColor)))))

(fn GetMergedColor
  (bind _merged_color (Variables|Colors|GetMerged%20Color))
  (bind (_r _g _b) (Math|Color|BreakColor _merged_color))
  (return (Math|Color|MakeColor (Math|Float|Clamp(Float) _r) (Math|Float|Clamp(Float) _g) (Math|Float|Clamp(Float) _b))))

(fn RecalculateColors
  (params (InputPin :type A%20Laser%20Object%20Reference))
  (Utilities|FlowControl|Sequence
    (:then_0
      (if (Utilities|Enum|Equal(Enum) (Variables|Colors|GetUsedColor) "NewEnumerator2")
        (Variables|Colors|SetMerged%20Color "")
        (for _array_element (Variables|Strorage|GetLasersInQueue)
          (Variables|Colors|SetMerged%20Color (+ (Variables|/Game/Lasers(LIghtPuzzle)/Blueprints/BuildingBlocks/A_Laser.A_Laser_C|GetColorOverride _array_element) (Variables|Colors|GetMerged%20Color))))))
    (:then_1
      (CallFunction|ComponentColorChange InputPin)
      (if (CallFunction|CanActivate)
        (CallFunction|CEActivateOverride)
        (else
          (CallFunction|CEDeactivateOverride))))))

(fn ComponentColorChange
  (params (Modified :type A%20Laser%20Object%20Reference))
  (bind _array_element (Utilities|ForEachComponent)
    (:LoopBody
      (Class|BPILasers|IntermediateChange(Message) _array_element Modified))))

(fn IsLaserFiltered
  (params (Laser%20In :type A%20Laser%20Object%20Reference))
  (return (Utilities|Array|ContainsItem (Variables|Lasers|GetLaserFilter) (Utilities|SetAlphato1 (Variables|/Game/Lasers(LIghtPuzzle)/Blueprints/BuildingBlocks/A_Laser.A_Laser_C|GetColorOverride Laser%20In)))))

(fn CanActivate
  (bind _output_get (LocalVariables|SetL-FilteredLasers (Variables|Strorage|GetFilteredLasers)))
  (if (Utilities|Array|IsEmpty _output_get)
    (return false)
    (elif (Utilities|Array|IsEmpty (Variables|Lasers|GetLaserRules))
      (return true)
      (elif (> (Utilities|Array|Length (Variables|Lasers|GetLaserRules)) (Utilities|Array|Length (LocalVariables|GetL-FilteredLasers)))
        (return false)
        (elif (Variables|Colors|GetCanMergeColor)
          (for _array_element (Variables|Lasers|GetLaserRules)
            (if (or (Utilities|ColorEqual :B _array_element) (CallFunction|DoesContainColor (CallFunction|GetMergedColor) _array_element))
              (Math|Integer|IncrementInt (LocalVariables|GetL-Counter))))
          (return (== (Utilities|Array|Length (Variables|Lasers|GetLaserRules)) (LocalVariables|GetL-Counter)))
          (else
            (for _array_element_2 (Variables|Lasers|GetLaserRules)
              (bind _output_get_2 (LocalVariables|SetL-Current%20Color _array_element_2))
              (if (not (Utilities|ColorEqual _output_get_2))
                (bind (_array_element_3 _array_index) (Utilities|Array|ForEachLoopwithBreak (LocalVariables|GetL-FilteredLasers) :!label _label)
                  (:LoopBody
                    (if (CallFunction|DoesContainColor (Variables|/Game/Lasers(LIghtPuzzle)/Blueprints/BuildingBlocks/A_Laser.A_Laser_C|GetColorOverride _array_element_3) (LocalVariables|GetL-Current%20Color))
                      (Math|Integer|IncrementInt (LocalVariables|GetL-Counter)
                        (:%20%20
                          (Utilities|Array|RemoveIndex (LocalVariables|GetL-FilteredLasers) _array_index)
                          (goto _label Break))))))
                (else
                  (Math|Integer|IncrementInt (LocalVariables|GetL-Counter)))))
            (return (== (Utilities|Array|Length (Variables|Lasers|GetLaserRules)) (LocalVariables|GetL-Counter)))))))))

(fn DoesContainColor
  (params (Input :type Linear%20Color%20Structure) (Condition :type Linear%20Color%20Structure))
  (bind (_r _g _b) (Utilities|Struct|BreakLinearColor Condition))
  (bind (_r_2 _g_2 _b_2) (Utilities|Struct|BreakLinearColor Input))
  (if (Variables|Colors|GetUseColorValue)
    (return (Math|Boolean|ANDBoolean (>= _r_2 _r) (>= _g_2 _g) (>= _b_2 _b)))
    (else
      (return (Utilities|ColorEqual Input Condition)))))

(fn StartTimer
  (params (ExternalTimer :type Boolean))
  (if (Class|KismetSystemLibrary|TimerExistsHandle (Variables|Timer|GetTimerHandle))
    (Utilities|Time|ClearandInvalidateTimerbyHandle (Variables|Timer|GetTimerHandle)))
  (if ExternalTimer
    (bind _returnvalue (Utilities|Time|SetTimerbyEvent (EventDispatchers|CreateEvent :!event ExternalUpdateTimer) (Variables|Timer|GetSubstep) true))
    (Variables|Timer|SetTimerHandle _returnvalue)
    (else
      (bind _returnvalue_2 (Utilities|Time|SetTimerbyEvent (EventDispatchers|CreateEvent :!event UpdateTimer) (Variables|Timer|GetSubstep) true))
      (Variables|Timer|SetTimerHandle _returnvalue_2))))

(fn UpdateTimer
  (if (select (Variables|Timer|GetReverseTimer) (<= (Variables|Timer|GetTimerAlpha) 0.0) (>= (Variables|Timer|GetTimerAlpha) 1.0))
    (Utilities|Time|ClearandInvalidateTimerbyHandle (Variables|Timer|GetTimerHandle))
    (if (Variables|Timer|GetReverseTimer)
      (CallFunction|CETimerFinishedDeactivate)
      (else
        (CallFunction|CETimerFinishedActivate)))
    (else
      (Variables|Timer|SetTimerAlpha (+ (* (* (/ 1.0 (Variables|Timer|GetDuration)) (Variables|Timer|GetSubstep)) (Math|Float|SelectFloat -1.0 1.0 (Variables|Timer|GetReverseTimer))) (Variables|Timer|GetTimerAlpha)))
      (Default|CallUpdateHandler (Variables|Timer|GetTimerAlpha)))))

(fn AreAllCompsActivated
  (for _array_element (Variables|Strorage|GetLinkedExternalComps)
    (if (not (Variables|/Game/Lasers(LIghtPuzzle)/Blueprints/BuildingBlocks/AC_External.AC_External_C|GetIsCompActivated _array_element))
      (return false)))
  (return true))

(fn ExternalUpdateTimer
  (if (select (Variables|Timer|GetReverseTimer) (<= (Variables|Timer|GetTimerAlpha) 0.0) (>= (Variables|Timer|GetTimerAlpha) 1.0))
    (Utilities|Time|ClearandInvalidateTimerbyHandle (Variables|Timer|GetTimerHandle))
    (if (Variables|Timer|GetReverseTimer)
      (CallFunction|CEExtTimerDeactivate)
      (else
        (CallFunction|CEExtTimerActivate)))
    (else
      (Variables|Timer|SetTimerAlpha (+ (* (* (/ 1.0 (Variables|Timer|GetDuration)) (Variables|Timer|GetSubstep)) (Math|Float|SelectFloat -1.0 1.0 (Variables|Timer|GetReverseTimer))) (Variables|Timer|GetTimerAlpha)))
      (Default|CallUpdateHandler (Variables|Timer|GetTimerAlpha)))))