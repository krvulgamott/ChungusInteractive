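; AC_External is a laser light puzzle component that relays activate, deactivate and update signals between AC_Handler-driven actors through its own dispatchers.
; Normally it tracks instigator states in NecessaryActors, activating only when all are true and deactivating when any one drops.
; InvertControl skips that check and just sets IsCompActivated before broadcasting.
; BeginPlay loops over TargetActors with empty bodies, as the handler registration and binding nodes are disconnected.
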(event EventBeginPlay
  (if (Variables|Default|GetInvertControl)
    (for _array_element (Variables|Default|GetTargetActors)
      _)
    (else
      (for _array_element_2 (Variables|Default|GetTargetActors)
        _))))

(fn ActivateThis
  (params (Instigator :type AC%20Handler%20Object%20Reference))
  (if (Variables|Default|GetInvertControl)
    (Variables|Default|SetIsCompActivated true)
    (Default|CallExternalActivate (Variables|Default|GetApplyConditions))
    (else
      (Utilities|FlowControl|Sequence
        (:then_0
          (Utilities|Map|Add (Variables|Default|GetNecessaryActors) Instigator true))
        (:then_1
          (if (CallFunction|AllActorActive)
            (Default|CallExternalActivate (Variables|Default|GetApplyConditions))))))))

(fn DeactivateThis
  (params (Instigator :type AC%20Handler%20Object%20Reference))
  (if (Variables|Default|GetInvertControl)
    (Variables|Default|SetIsCompActivated false)
    (Default|CallExternalDeactivate (Variables|Default|GetApplyConditions))
    (else
      (Utilities|Map|Add (Variables|Default|GetNecessaryActors) Instigator false)
      (Default|CallExternalDeactivate (Variables|Default|GetApplyConditions)))))

(fn UpdateThis
  (params (Alpha :type Float%20%28double-precision%29))
  (Default|CallExternalUpdate Alpha))

(fn AllActorActive
  (bind _keys (Utilities|Map|Keys (Variables|Default|GetNecessaryActors)))
  (for _array_element _keys
    (if (not (.Value (Utilities|Map|Find (Variables|Default|GetNecessaryActors) _array_element)))
      (return false)))
  (return true))