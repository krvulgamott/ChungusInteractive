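; AC_Bounce is an actor component for the laser light puzzle that reflects incoming lasers.
; Each hitting laser gets its own spawned SC_Emitter, stored in a map, which is moved while the hit updates and destroyed when it stops.
; Emitters can inherit the incoming laser's color.
; Forced activation and deactivation replay start and stop hits over the owner AC_Handler's filtered lasers.
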(event EventBeginPlay
  (bind _returnvalue (Components|GetOwner))
  (bind _returnvalue_2 (Actor|GetComponentbyClass _returnvalue "/Game/Lasers(LIghtPuzzle)/Blueprints/BuildingBlocks/AC_Handler.AC_Handler_C"))
  (Utilities|IsValid _returnvalue_2
    (:Is%20Valid
      (Variables|Default|SetOwningHandler _returnvalue_2))))

(event EventIntermediateChange
  (params (Modified :type A%20Laser%20Object%20Reference))
  (bind _values (Utilities|Map|Values (Variables|Default|GetEmitterBounceMap)))
  (for _array_element _values
    (Default|SetLaserColor _array_element)))

(event EventLaserStopHitting
  (params (Input :type A%20Laser%20Object%20Reference))
  (CallFunction|RemoveLaser Input))

(event EventLaserUpdateHitting
  (params (Input :type A%20Laser%20Object%20Reference) (Hit%20Info :type Hit%20Result%20Structure))
  (bind (_location _rotation) (Utilities|MirrorLocationRotation Hit%20Info))
  (bind _emitterbouncemap (Variables|Default|GetEmitterBounceMap))
  (bind (_value _returnvalue) (Utilities|Map|Find _emitterbouncemap Input))
  (if _returnvalue
    (Transformation|SetWorldLocationAndRotation _value _location _rotation false false)))

(event EventForceDeactivation
  (params (ApplyConditions :type Boolean))
  (for _array_element (Variables|/Game/Lasers(LIghtPuzzle)/Blueprints/BuildingBlocks/AC_Handler.AC_Handler_C|GetFilteredLasers (Variables|Default|GetOwningHandler))
    (CallFunction|LaserStopHitting _array_element)))

(event EventForceActivation
  (params (ApplyConditions :type Boolean))
  (for _array_element (Variables|/Game/Lasers(LIghtPuzzle)/Blueprints/BuildingBlocks/AC_Handler.AC_Handler_C|GetFilteredLasers (Variables|Default|GetOwningHandler))
    (if (.ReturnValue (Default|GetHitbyHandler _array_element (Variables|Default|GetOwningHandler)))
      (CallFunction|LaserStartHitting _array_element (.Value (Default|GetHitbyHandler _array_element (Variables|Default|GetOwningHandler)))))))

(event EventLaserStartHitting
  (params (Input :type A%20Laser%20Object%20Reference) (Hit%20Info :type Hit%20Result%20Structure))
  (Utilities|IsValid Input
    (:Is%20Valid
      (if (not (Utilities|Map|Contains (Variables|Default|GetEmitterBounceMap) Input))
        (CallFunction|SpawnLaser Input Hit%20Info)))))

(fn SpawnLaser
  (params (Laser%20In :type A%20Laser%20Object%20Reference) (Hit%20Info :type Hit%20Result%20Structure))
  (bind _returnvalue (Components|GetOwner))
  (bind _returnvalue_2 (Transformation|GetActorTransform _returnvalue))
  (bind (_location _rotation) (Utilities|MirrorLocationRotation Hit%20Info))
  (bind _returnvalue_3 (Game|AddComponentbyClass (Components|GetOwner) "/Game/Lasers(LIghtPuzzle)/Blueprints/BuildingBlocks/SC_Emitter.SC_Emitter_C" false (Math|Transform|MakeTransform (Math|Transform|InverseTransformLocation _returnvalue_2 _location) (Math|Transform|InverseTransformRotation _returnvalue_2 _rotation) "1.000000,1.000000,1.000000")))
  (Utilities|Map|Add (Variables|Default|GetEmitterBounceMap) Laser%20In _returnvalue_3)
  (if (Variables|Default|GetUseBounceColor)
    (Variables|/Game/Lasers(LIghtPuzzle)/Blueprints/BuildingBlocks/SC_Emitter.SC_Emitter_C|SetOverride%20Color _returnvalue_3 (Variables|/Game/Lasers(LIghtPuzzle)/Blueprints/BuildingBlocks/A_Laser.A_Laser_C|GetColorOverride Laser%20In))
    (Variables|/Game/Lasers(LIghtPuzzle)/Blueprints/BuildingBlocks/SC_Emitter.SC_Emitter_C|SetUseOverride _returnvalue_3 true))
  (Default|SetLaserColor _returnvalue_3)
  (Default|ActivateLaser _returnvalue_3))

(fn RemoveLaser
  (params (InputPin :type A%20Laser%20Object%20Reference))
  (bind _emitterbouncemap (Variables|Default|GetEmitterBounceMap))
  (bind (_value _returnvalue) (Utilities|Map|Find _emitterbouncemap InputPin))
  (if _returnvalue
    (bind _output_get (LocalVariables|SetL-RemoveItem _value))
    (Default|LaserStopHitting _output_get)
    (Default|DestorySelf (LocalVariables|GetL-RemoveItem))
    (Utilities|Map|Remove (Variables|Default|GetEmitterBounceMap) InputPin)))