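; BP_RisingWater is a water actor that rises and lowers in response to an assigned shrine.
; On BeginPlay it stores its scale and binds to the shrine's activated and deactivated events, or prints a warning if none is set.
; Two separate timelines drive only Z scale to fake the water level.
; A Niagara effect toggles once when raising starts, but on every timeline update while lowering.
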(event Custom|Raise%20Water
  ;[1 1 0] Check details for multiple shrines.
  (Components|Activation|ToggleActive (Variables|/Script/Niagara.NiagaraActor|GetNiagaraComponent (Variables|Default|GetVFX)))
  (bind _floattrack (Timeline|RaiseWaterTimeline Play)
    (:Update
      (Transformation|SetActorScale3D (Math|Vector|MakeVector (.x (stale EventBeginPlay _output_get)) (.y (stale EventBeginPlay _output_get)) _floattrack)))))

(event Custom|Lower%20Water
  ;[1 1 0] Check details for multiple shrines.
  (bind _floattrack (Timeline|LowerWaterTimeline Play)
    (:Update
      (Transformation|SetActorScale3D (Math|Vector|MakeVector (.x (stale EventBeginPlay _output_get)) (.y (stale EventBeginPlay _output_get)) _floattrack))
      (Components|Activation|ToggleActive (Variables|/Script/Niagara.NiagaraActor|GetNiagaraComponent (Variables|Default|GetVFX))))))

(event EventBeginPlay
  (bind _refshrine (Variables|Default|GetRefShrine))
  ;[1 1 0] Check details for multiple shrines.
  (bind _output_get (Variables|Default|SetOriginalScale (Transformation|GetActorScale3D)))
  (Utilities|IsValid _refshrine
    (:Is%20Valid
      (EventDispatchers|BindEventtoOnActivated _refshrine (delegate Custom|Raise%20Water))
      (EventDispatchers|BindEventtoOnDeactivated _refshrine (delegate Custom|Lower%20Water)))
    (:Is%20Not%20Valid
      (Development|PrintString "Assign Platform to Shrine in Editor"))))

(fn ConstructionScript)