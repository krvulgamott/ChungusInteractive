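; BP_Shrine_Water is a water shrine actor that toggles between active and inactive when interacted with.
; Interact checks IsActive, runs the matching activate or deactivate event, then calls OnActivated or OnDeactivated to broadcast the change.
; Those events set the flag and swap TempItem's material between temporary green and red as placeholder feedback.
; AddItem is a stub that always returns false.
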(event Custom|Activate%20Shrine
  ;[0.15 0.15 0.15 0.5] Activate/Deactivate Shrine. Changes the shrine to look active or inactive.
  (Variables|Default|SetIsActive? true)
  (Rendering|Material|SetMaterial (Variables|Default|GetTemp_Item) 0 "/Game/Materials/Temp_Green.Temp_Green"))

(event Custom|Deactivate%20Shrine
  ;[0.15 0.15 0.15 0.5] Activate/Deactivate Shrine. Changes the shrine to look active or inactive.
  (Variables|Default|SetIsActive? false)
  (Rendering|Material|SetMaterial (Variables|Default|GetTemp_Item) 0 "/Game/Materials/Temp_Red.Temp_Red"))

(event EventBeginPlay)

(event Collision|EventActorBeginOverlap
  (params (OtherActor :type Actor%20Object%20Reference)))

(event EventTick
  (params (DeltaSeconds :type Float%20%28single-precision%29)))

(event EventInteract
  (params (Interactor :type BP%202D%20Char%20Object%20Reference))
  ;[0.15 0.15 0.15 0.5] Logic for shrine interaction
  (if (Variables|Default|GetIsActive?)
    (CallFunction|DeactivateShrine)
    (Default|CallOnDeactivated)
    (else
      (CallFunction|ActivateShrine)
      (Default|CallOnActivated))))

(fn ConstructionScript)

(fn AddItem
  (params (Item :type Actor%20Object%20Reference))
  (return false))