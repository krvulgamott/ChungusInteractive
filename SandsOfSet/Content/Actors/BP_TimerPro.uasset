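; BP_TimerPro is an interactable timer shrine actor that spawns a platform when used.
; Interact spawns BP_SpawnPlatform2 at a hard-coded transform and prints a debug "Start", with no timing logic present.
; ActivateShrine and DeactivateShrine are empty, as the active toggle, red/green material swap and TargetPoint-based spawn nodes are disconnected.
; AddItem is a stub that always reports no sand.
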(event Custom|Activate%20Shrine
  ;[0.15 0.15 0.15 0.5] Activate/Deactivate Shrine. Changes the shrine to look active or inactive.
)

(event Custom|Deactivate%20Shrine
  ;[0.15 0.15 0.15 0.5] Activate/Deactivate Shrine. Changes the shrine to look active or inactive.
)

(event EventBeginPlay)

(event Collision|EventActorBeginOverlap
  (params (OtherActor :type Actor%20Object%20Reference)))

(event EventTick
  (params (DeltaSeconds :type Float%20%28single-precision%29)))

(event EventInteract
  (params (Interactor :type BP%20Third%20Person%20Character%20Object%20Reference))
  (Game|SpawnActorfromClass "/Game/LevelOnePuzzles/Timer/BP_SpawnPlatform2.BP_SpawnPlatform2_C" (Math|Transform|MakeTransform "440.000000,-500.000000,60.000000") "Undefined" "MultiplyWithRoot" 0 0)
  (Development|PrintString "Start"))

(fn ConstructionScript)

(fn AddItem
  (params (Item :type Actor%20Object%20Reference))
  (return 0.0 false))