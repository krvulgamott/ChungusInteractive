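; BP_Pedestal is an interactable pedestal that stores sand taken from the interacting player and gives it back.
; Interact moves exactly ValueCap from the player's PlayerSand into StoredSand when the player has enough and the pedestal is not full, calling Filled.
; Otherwise it returns any stored sand and calls Emptied, even if already empty.
; Each interaction prints both totals; AddItem is a stub returning false.
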(event EventBeginPlay
  (Variables|Default|SetStoredSand 0.0))

(event Collision|EventActorBeginOverlap
  (params (OtherActor :type Actor%20Object%20Reference)))

(event EventTick
  (params (DeltaSeconds :type Float%20%28single-precision%29)))

(event EventInteract
  (params (Interactor :type BP%202D%20Char%20Object%20Reference))
  (bind _valuecap (Variables|Default|GetValueCap))
  (if (>= (Variables|/Game/MainChar/BP_2DChar.BP_2DChar_C|GetPlayerSand Interactor) _valuecap)
    (if (== (Variables|Default|GetStoredSand) _valuecap)
      (Variables|/Game/MainChar/BP_2DChar.BP_2DChar_C|SetPlayerSand Interactor (+ (Variables|/Game/MainChar/BP_2DChar.BP_2DChar_C|GetPlayerSand Interactor) (Variables|Default|GetStoredSand)) :!label _label)
      (Variables|Default|SetStoredSand 0.0)
      (Default|CallEmptied)
      (else
        (Variables|Default|SetStoredSand _valuecap)
        (Variables|/Game/MainChar/BP_2DChar.BP_2DChar_C|SetPlayerSand Interactor (- (Variables|/Game/MainChar/BP_2DChar.BP_2DChar_C|GetPlayerSand Interactor) _valuecap))
        (Default|CallFilled)))
    (else
      (goto _label)))
  (Development|PrintString (Utilities|String|ToString(Text) (Utilities|Text|FormatText "Player has {Player Sand} and Pedestal has {Stored Sand}." (Variables|/Game/MainChar/BP_2DChar.BP_2DChar_C|GetPlayerSand Interactor) (Variables|Default|GetStoredSand)))))

(fn ConstructionScript)

(fn AddItem
  (params (Item :type Actor%20Object%20Reference))
  (return false))