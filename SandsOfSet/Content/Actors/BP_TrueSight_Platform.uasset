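; True Sight platform actor that starts hidden and non-collidable until revealed.
; ActivateTrueSight toggles Cube visible and enables Box collision, then reverses both after a ten-second Delay.
; A repeat call while CanCollide is set drops collision early but leaves visibility untouched.
; Debug prints report a five-second wait, unlike the actual delay, and Cube is marked for replacement by a final asset.
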(event Custom|Activate%20TrueSight
  (if (Variables|Default|GetCanCollide?)
    (Collision|SetCollisionEnabled (Variables|Default|GetBox) "NoCollision")
    (Development|PrintString "Can't Collide (Wait 5s)")
    (Variables|Default|SetCanCollide? false)
    (else
      (Rendering|ToggleVisibility (Variables|Default|GetCube) false)
      (Collision|SetCollisionEnabled (Variables|Default|GetBox) "QueryAndPhysics")
      (Development|PrintString "Can Collide (Wait 5s)")
      (Variables|Default|SetCanCollide? true)
      (Utilities|FlowControl|Delay 1e+01)
      (Rendering|ToggleVisibility (Variables|Default|GetCube) false)
      (Collision|SetCollisionEnabled (Variables|Default|GetBox) "NoCollision")
      (Variables|Default|SetCanCollide? false))))

(event EventBeginPlay
  ;[0.894 0.8505 0 0.5] Need to change target when given asset
  (Rendering|SetVisibility (Variables|Default|GetCube) false false)
  (Collision|SetCollisionEnabled (Variables|Default|GetBox) "NoCollision")
  (Variables|Default|SetCanCollide? false))

(event Collision|EventActorBeginOverlap
  (params (OtherActor :type Actor%20Object%20Reference)))

(event EventTick
  (params (DeltaSeconds :type Float%20%28single-precision%29)))

(fn ConstructionScript)